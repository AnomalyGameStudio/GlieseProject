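; Blueprint function library with camera helpers that switch the first player controller's view to another camera or back to the player.
; MoveToNewCamera blends the view target to a given camera with cubic easing over a supplied time.
; ResetCameraToPlayer blends the view back to the player reference using the default blend function.
; Both validate their inputs and return whether the blend was started.
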(fn `MoveToNewCamera`
  (params (PlayerRef :type "/Game/GlieseProject/Blueprints/Characters/SideScrollerCharacter Object Reference") (NewCamera :type "CameraActor Object Reference") (BlendTime :type "Float (double-precision)"))
  (returns (`Success?` :type Boolean))
  (locals (LocalPlayer :type "/Game/GlieseProject/Blueprints/Characters/SideScrollerCharacter Object Reference") (LocalCamera :type "CameraActor Object Reference") (LocalBlendTime :type "Float (double-precision)" :default 1.0))
  (set `local.LocalPlayer` PlayerRef)
  (set `local.LocalCamera` NewCamera)
  (set `local.LocalBlendTime` BlendTime)
  (if (and (`KismetSystemLibrary.IsValid` (`local.LocalPlayer`)) (`KismetSystemLibrary.IsValid` (`local.LocalCamera`)))
    (`PlayerController.SetViewTargetWithBlend` (`GameplayStatics.GetPlayerController` (`local.LocalPlayer`)) (`local.LocalCamera`) (`local.LocalBlendTime`) "VTBlend_Cubic" 0.0 false)
    (return true)
    (else
      (return false))))

(fn `ResetCameraToPlayer`
  (params (PlayerRef :type "/Game/GlieseProject/Blueprints/Characters/SideScrollerCharacter Object Reference") (BlendTime :type "Float (double-precision)"))
  (returns (`Success?` :type Boolean))
  (locals (LocalPlayer :type "/Game/GlieseProject/Blueprints/Characters/SideScrollerCharacter Object Reference") (LocalBlendTime :type "Float (double-precision)" :default 1.0))
  (bind _localplayer (`local.LocalPlayer`))
  (set `local.LocalPlayer` PlayerRef)
  (set `local.LocalBlendTime` BlendTime)
  (`/Engine/EditorBlueprintResources/StandardMacros.IsValid` (`local.LocalPlayer`)
    (:`Is Valid`
      (`PlayerController.SetViewTargetWithBlend` (`GameplayStatics.GetPlayerController` _localplayer) _localplayer (`local.LocalBlendTime`) "VTBlend_Linear" 0.0 false)
      (return true))
    (:`Is Not Valid`
      (return false))))