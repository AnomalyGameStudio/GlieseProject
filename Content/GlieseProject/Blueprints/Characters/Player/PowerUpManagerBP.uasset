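; PowerUpManagerBP is an actor that unlocks and triggers the player character's power-ups, Double Jump and Blink.
; AddPowerUp grants each ability once, with Double Jump raising JumpMaxCount, and adds an entry to the power-up menu widget on every call.
; UsePowerUp handles only Blink, a swept forward teleport gated by a timer-based cooldown.
; SelectPowerUp is an empty stub.
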(event `Blink`
  (bind _playercharacter (`self.PlayerCharacter`))
  ;[1 1 1] Blink Power Up
  (if (and (`self.CanBlink?`) (`self.Blink?`))
    (`self.K2_SetActorLocation` (`self.PlayerCharacter`) (+ (`self.K2_GetActorLocation` _playercharacter) (* (`KismetMathLibrary.GetForwardVector` (`self.K2_GetActorRotation` _playercharacter)) (`self.BlinkDistance`))) true true)
    (`KismetSystemLibrary.K2_SetTimerDelegate` (delegate `StartCooldown`) (`self.BlinkCooldown`))
    (set `self.CanBlink?` false)))

(event `StartCooldown`
  ;[1 1 1] Blink Power Up
  (set `self.CanBlink?` true))

(event `UsePowerUp`
  (params (PowerUp :type "/Game/GlieseProject/Blueprints/Enums/e_PowerUpTypes Enum"))
  (switch `/Game/GlieseProject/Blueprints/Enums/e_PowerUpTypes` PowerUp
    (:`NewEnumerator1`
      (`self.Blink`))))

(event `SelectPowerUp`)

(fn `AddBlink`
  (if (not (`self.Blink?`))
    (bind _output_get (set `self.Blink?` true))
    (set `self.CanBlink?` _output_get))
  (return))

(fn `AddDoubleJump`
  (if (`self.DoubleJump?`)
    (return)
    (else
      (set `self.DoubleJump?` true)
      (set `Character.JumpMaxCount` (+ (`Character.JumpMaxCount` (`self.PlayerCharacter`)) 1) (`self.PlayerCharacter`))
      (return))))

(fn `AddPowerUp`
  (params (PowerUp :type "/Game/GlieseProject/Blueprints/Enums/e_PowerUpTypes Enum"))
  (switch `/Game/GlieseProject/Blueprints/Enums/e_PowerUpTypes` PowerUp
    (:`NewEnumerator0`
      (`self.AddDoubleJump`))
    (:`NewEnumerator1`
      (`self.AddBlink`)))
  (`/Game/GlieseProject/Widgets/PowerUpMenuWidget.AddPowerUpEntry` (`/Game/GlieseProject/Widgets/MainWidget.PowerUpMenuWidget` (`/Game/GlieseProject/Blueprints/Characters/SideScrollerCharacter.MainWidget` (`self.PlayerCharacter`))) PowerUp))

(fn `UserConstructionScript`)