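; Master NPC base character that shows a name widget near the player and handles dialogue on interaction, granting its quest first if the player lacks it.
; Regular NPCs cycle through short timed text bubbles, then notify the player's QuestManager.
; Important NPCs run a cutscene-style conversation: screen fades, player movement is disabled, the camera blends per line and lines go through the player's DialogueManager.
; Ending the conversation restores camera and movement.
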(event `self.ReceiveBeginPlay`
  ;[1 1 1] Event Begin Play
  (`self.UpdateName`))

(event `/Game/GlieseProject/Interfaces/i_Interactable.OnEnterPlayerRadius`
  ;[1 1 1] On Enter Player Radius
  (set `self.IsPlayerRadius?` true)
  (if (not (`self.IsTalking?`))
    (`SceneComponent.SetVisibility` (`self.NpcWidget`) true false)))

(event `End Conversation`
  ;[1 1 1] Event End Conversation
  (set `self.CurrentDialogueIndex` 0)
  (`self.FadeToBlack` false
    (:`Completed`
      (`SceneComponent.SetVisibility` (`self.NpcWidget`) (`self.IsPlayerRadius?`) false)
      (`self.ResetCamera`)
      (`self.FadeToBlack` true
        (:`Then`
          (`CharacterMovementComponent.SetMovementMode` (`Character.CharacterMovement` (`self.PlayerCharacterRef`)) "MOVE_Walking" 0))
        (:`Completed`
          (set `self.IsTalking?` false))))))

(event `/Game/GlieseProject/Interfaces/i_Interactable.OnLeavePlayerRadius`
  ;[1 1 1] On Leave Player Radius
  (set `self.IsPlayerRadius?` false)
  (if (not (`self.IsTalking?`))
    (`SceneComponent.SetVisibility` (`self.NpcWidget`) false false)))

(event `OnDialogueEnd`
  (params (Index :type Integer))
  ;[1 1 1] Event OnDialogueEnd
  (if (== (`KismetArrayLibrary.Array_LastIndex` (`self.ImportantDialogues`)) (`self.CurrentDialogueIndex`))
    (`self.End Conversation`)
    (else
      (`/Engine/EditorBlueprintResources/StandardMacros.IncrementInt` (`self.CurrentDialogueIndex`)
        (:`  `
          (`self.HandleCamera`)
          (`self.ShowNextImportanteDialogue` (`self.CurrentDialogueIndex`)))))))

(event `AddDialogue`
  ;[1 1 1] Add Dialogue Event
  (set `self.IsTalking?` true)
  (`self.ShowDialogue` (`KismetArrayLibrary.Array_Get` (`self.Dialogues`) (`self.CurrentDialogueIndex`)))
  (`KismetSystemLibrary.Delay` 1.0)
  (`self.OnSimpleDialogFinished`))

(event `OnSimpleDialogFinished`
  (bind _currentdialogueindex (`self.CurrentDialogueIndex`))
  ;[1 1 1] OnSimpleDialogFinished Event
  (set `self.CurrentDialogueIndex` (select `bool` (== _currentdialogueindex (`KismetArrayLibrary.Array_LastIndex` (`self.Dialogues`))) :`false` (+ _currentdialogueindex 1)))
  (`SceneComponent.SetVisibility` (`self.NpcWidget`) (`self.IsPlayerRadius?`) false)
  (`SceneComponent.SetVisibility` (`self.NpcText`) false false)
  (set `self.IsTalking?` false)
  (`/Game/GlieseProject/Blueprints/Actors/Bp_QuestManager.OnTalkToNpc` (`/Game/GlieseProject/Blueprints/Characters/SideScrollerCharacter.QuestManager` (`self.PlayerCharacterRef`)) (`GameplayStatics.GetObjectClass` self) (`self.NpcId`)))

(event `StartDialog`
  (params (PlayerChar :type "/Game/GlieseProject/Blueprints/Characters/SideScrollerCharacter Object Reference"))
  (bind _charactermovement (`Character.CharacterMovement` (`self.PlayerCharacterRef`)))
  ;[1 1 1] On Interact With
  (bind _output_get (set `self.PlayerCharacterRef` PlayerChar))
  (set `self.MainWidget` (`/Game/GlieseProject/Blueprints/Characters/SideScrollerCharacter.MainWidget` _output_get))
  (if (`self.IsImportant?`)
    (if (not (`self.IsTalking?`))
      (set `self.isTalking?` true)
      (set `self.CurrentDialogueIndex` 0)
      (`self.FadeToBlack` false
        (:`Then`
          (`CharacterMovementComponent.DisableMovement` _charactermovement)
          (`MovementComponent.StopMovementImmediately` _charactermovement))
        (:`Completed`
          (`SceneComponent.SetVisibility` (`self.NpcWidget`) false false)
          (`self.HandleCamera`)
          (`self.FadeToBlack` true
            (:`Completed`
              (`self.ShowNextImportanteDialogue` 0))))))
    (elif (not (`self.IsTalking?`))
      (`self.AddDialogue`))))

(event `/Game/GlieseProject/Interfaces/i_Interactable.OnInteractWith`
  (params (PlayerChar :type "/Game/GlieseProject/Blueprints/Characters/SideScrollerCharacter Object Reference"))
  (bind _hasquest (`self.HasQuest`))
  (bind _questmanager (`/Game/GlieseProject/Blueprints/Characters/SideScrollerCharacter.QuestManager` PlayerChar))
  (if (`KismetSystemLibrary.IsValidClass` (`self.HasQuest`))
    (if (`KismetArrayLibrary.Array_Contains` (`/Game/GlieseProject/Blueprints/Actors/Bp_QuestManager.AllQuestClasses` _questmanager) _hasquest)
      (`self.StartDialog` PlayerChar)
      (else
        (`/Game/GlieseProject/Blueprints/Actors/Bp_QuestManager.AddNewQuest` _questmanager _hasquest true)
        (`self.StartDialog` PlayerChar)))
    (else
      (`self.StartDialog` PlayerChar))))

(fn `HandleCamera`
  (bind (_spokentext _sendername _canbeskipped_ _skiptime _switchtonewcamera_ _newcamera _blendtime) (break `/Game/GlieseProject/Blueprints/Structures/s_DialogueInfo` (`KismetArrayLibrary.Array_Get` (`self.ImportantDialogues`) (`self.CurrentDialogueIndex`))))
  (if (and _switchtonewcamera_ (`KismetSystemLibrary.IsValid` _newcamera))
    (`PlayerController.SetViewTargetWithBlend` (`GameplayStatics.GetPlayerController` 0) _newcamera _blendtime "VTBlend_Cubic" 0.0 false)
    (return)
    (else
      (return))))

(fn `ResetCamera`
  (`PlayerController.SetViewTargetWithBlend` (`GameplayStatics.GetPlayerController` 0) (`self.PlayerCharacterRef`) 0.0 "VTBlend_Linear" 0.0 false)
  (return))

(fn `ShowDialogue`
  (params (Text :type Text))
  (`TextBlock.SetText` (`/Game/GlieseProject/Widgets/NpcText.Text` (cast `/Game/GlieseProject/Widgets/NpcText` (`WidgetComponent.GetUserWidgetObject` (`self.NpcText`)) :!pure true)) Text)
  (`SceneComponent.SetVisibility` (`self.NpcWidget`) false false)
  (`SceneComponent.SetVisibility` (`self.NpcText`) true false)
  (return))

(fn `ShowNextImportanteDialogue`
  (params (Index :type Integer))
  (bind _playercharacterref (`self.PlayerCharacterRef`))
  (`/Engine/EditorBlueprintResources/StandardMacros.IsValid` _playercharacterref
    (:`Is Valid`
      (`/Game/GlieseProject/Blueprints/Bp_DialogueManager.AddSimpleDialogue` (`/Game/GlieseProject/Blueprints/Characters/SideScrollerCharacter.DialogueManager` _playercharacterref) (`KismetArrayLibrary.Array_Get` (`self.ImportantDialogues`) (`self.CurrentDialogueIndex`)) Index))
    (:`Is Not Valid`
      _))
  (return))

(fn `UpdateName`
  (bind _asnpc_widget (cast `/Game/GlieseProject/Widgets/NpcWidget` (`WidgetComponent.GetUserWidgetObject` (`self.NpcWidget`)))
    (:`then`
      (`TextBlock.SetText` (`/Game/GlieseProject/Widgets/NpcWidget.NameText` _asnpc_widget) (`self.Name`)))
    (:`CastFailed`
      _))
  (return))

(fn `UserConstructionScript`)