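; Dialogue manager actor that shows one message at a time in the main HUD widget, which it creates on BeginPlay.
; AddSimpleDialogue ignores requests while a dialogue is active, displays sender and text, and marks it spoken after a fixed delay, revealing the skip prompt.
; Skippable lines accept input earlier.
; The continue command first completes an unfinished line, then hides it and notifies the player character with the dialogue index.
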(event `OnContinueDialogue`
  (set `self.WaitingForInput?` false)
  (`Widget.SetVisibility` (`/Game/GlieseProject/Widgets/MainWidget.MessageWidget` (`self.MainWidget`)) "Hidden")
  (set `self.DialogueFinished?` false)
  (set `self.CurrentDialogue?` false)
  (`/Game/GlieseProject/Blueprints/Characters/SideScrollerCharacter.OnDialogueFinished` (`self.PlayerCharacterRef`) (`self.CurrentDialogIndex`)))

(event `OnDialogueSpoken`
  (if (and (not (`self.DialogueFinished?`)) (`self.CurrentDialogue?`))
    (set `self.DialogueFinished?` true)
    (set `self.WaitingForInput?` true)
    (`Widget.SetVisibility` (`/Game/GlieseProject/Widgets/MessageWidget.SkipText` (`/Game/GlieseProject/Widgets/MainWidget.MessageWidget` (`self.MainWidget`))) "Visible")))

(event `HandleContinueCommand`
  (if (`self.WaitingForInput?`)
    (if (`self.CurrentDialogue?`)
      (if (`self.DialogueFinished?`)
        (`self.OnContinueDialogue`)
        (else
          (`self.OnDialogueSpoken`))))))

(event `AddSimpleDialogue`
  (params (Dialogue :type "/Game/GlieseProject/Blueprints/Structures/s_DialogueInfo Structure") (Index :type Integer))
  (bind (_spokentext _sendername _canbeskipped_ _skiptime) (break `/Game/GlieseProject/Blueprints/Structures/s_DialogueInfo` Dialogue))
  (if (not (`self.CurrentDialogue?`))
    (set `self.CurrentDialogue?` true)
    (set `self.CurrentDialogIndex` Index)
    (`/Game/GlieseProject/Widgets/MessageWidget.ShowNewMessage` (`/Game/GlieseProject/Widgets/MainWidget.MessageWidget` (`self.MainWidget`)) _sendername _spokentext)
    (`|ExecutionSequence`
      (:`then_0`
        (if _canbeskipped_
          (`KismetSystemLibrary.Delay` _skiptime)
          (set `self.WaitingForInput?` true)))
      (:`then_1`
        (`KismetSystemLibrary.Delay` 5.0)
        (`self.OnDialogueSpoken`)))))

(event `self.ReceiveBeginPlay`
  (bind _returnvalue (`|CreateWidget` "/Game/GlieseProject/Widgets/MainWidget.MainWidget_C"))
  (bind _output_get (set `self.MainWidget` _returnvalue))
  (`UserWidget.AddToViewport` _output_get 0))

(fn `UserConstructionScript`)